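; BP_CPawn is a player pawn that moves, looks around and grabs physics actors.
; Input axes drive movement along the player controller's forward and right vectors, plus yaw and pitch.
; Clicking the actor calls Grab with the grab distance, controller forward vector and eye viewpoint location.
; Helpers return its name and position or increment a counter, with either a printout or a delay.
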(event MouseInput|EventActorOnClicked
  (params (ButtonPressed :type Key%20Structure :default "None"))
  ;[1 1 1] Grab Actor (Physics Actor)
  (Class|Grab|Grab (Variables|Default|GetGrab) (Variables|Default|GetGrabDistance) (Transformation|GetActorForwardVector (Game|GetPlayerController 0)) (Math|Conversions|ToTransform(Vector) (.OutLocation (Actor|GetActorEyesViewPoint)))))

(event Input|AxisEvents|InputAxisLeft/Right
  (params (AxisValue :type Float%20%28single-precision%29))
  ;[1 1 1] Movement
  (Pawn|Input|AddMovementInput (Transformation|GetActorRightVector (Game|GetPlayerController 0)) AxisValue false))

(event Input|AxisEvents|InputAxisForward/Backward
  (params (AxisValue :type Float%20%28single-precision%29))
  ;[1 1 1] Movement
  (Pawn|Input|AddMovementInput (Transformation|GetActorForwardVector (Game|GetPlayerController 0)) AxisValue false))

(event Input|AxisEvents|InputAxisTurn
  (params (AxisValue :type Float%20%28single-precision%29))
  ;[1 1 1] Movement
  (Pawn|Input|AddControllerYawInput AxisValue))

(event Input|AxisEvents|InputAxisLookUp
  (params (AxisValue :type Float%20%28single-precision%29))
  ;[1 1 1] Movement
  (Pawn|Input|AddControllerPitchInput AxisValue))

(fn ConstructionScript)

(fn FctIncrement
  (bind _output_get (Variables|Default|Setinc (+ (Variables|Default|Getinc) 1)))
  (Development|PrintString (Utilities|String|ToString(Integer) _output_get)))

(fn ReturnName
  (return (Utilities|GetObjectName self)))

(fn ReturnPosition
  (return (Transformation|GetActorLocation self)))